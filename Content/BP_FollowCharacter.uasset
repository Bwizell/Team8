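; Shared camera actor for a two-player side-on game that becomes the view target shortly after BeginPlay and follows both characters.
; Each tick it sits at their X/Z midpoint, raised slightly, and shifts along Y as their X separation grows.
; It also gives the lower-X character a slipstream walk-speed boost proportional to the gap, unless zapped.
; A one-shot two-minute timer deducts a coin penalty from both players.
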(event Custom|CustomEvent
  ;[1 1 1] Timer Penalty
  (bind _asbp_character_1 (Utilities|Casting|CastToBP_Character1 (Game|GetPlayerCharacter 0)))
  (Variables|/Game/OurContent/Blueprints/BP_Character1.BP_Character1_C|SetCoins1 _asbp_character_1 (- (Variables|/Game/OurContent/Blueprints/BP_Character1.BP_Character1_C|GetCoins1 _asbp_character_1) 2e+02))
  (bind _asbp_character_2 (Utilities|Casting|CastToBP_Character2 (Variables|Default|GetPlayer2)))
  (Variables|/Game/OurContent/Blueprints/BP_Character2.BP_Character2_C|SetCoins2 _asbp_character_2 (- (Variables|/Game/OurContent/Blueprints/BP_Character2.BP_Character2_C|GetCoins2 _asbp_character_2) 2e+02)))

(event Collision|EventActorBeginOverlap
  (params (OtherActor :type Actor%20Object%20Reference)))

(event EventTick
  (params (DeltaSeconds :type Float%20%28single-precision%29))
  (bind _returnvalue (Transformation|GetActorLocation))
  (bind _returnvalue_2 (Transformation|GetActorLocation))
  (bind _returnvalue_3 (Transformation|GetActorLocation))
  (bind _player1 (Variables|Default|GetPlayer1))
  (bind _player2 (Variables|Default|GetPlayer2))
  (bind _player1_2 (Variables|Default|GetPlayer1))
  (bind _player2_2 (Variables|Default|GetPlayer2))
  (bind _fixed_y (Variables|Default|GetFixed%20Y))
  (bind _returnvalue_4 (Transformation|GetActorLocation _player1))
  (bind _returnvalue_5 (Transformation|GetActorLocation _player2))
  ;[1 1 1] Follow Inbetween The Two Character
  (Utilities|IsValid _player1
    (:Is%20Valid
      (Transformation|SetActorLocation (Math|Vector|MakeVector (/ (+ (.x _returnvalue_4) (.x _returnvalue_5)) 2.0) (.y (Transformation|GetActorLocation)) (+ 2e+02 (/ (+ (.z _returnvalue_4) (.z _returnvalue_5)) 2.0))) false false)
      (if (< (.x (Transformation|GetActorLocation (Variables|Default|GetPlayer1))) (.x (Transformation|GetActorLocation (Variables|Default|GetPlayer2))))
        (bind _output_get (Variables|Default|SetDistance (- (.x (Transformation|GetActorLocation (Variables|Default|GetPlayer2))) (.x (Transformation|GetActorLocation (Variables|Default|GetPlayer1))))))
        (if (> _output_get 3e+02)
          (bind _output_get_2 (Variables|Default|SetYOffSet (/ _output_get 2.0)))
          (else
            (bind _output_get_3 (Variables|Default|SetYOffSet _fixed_y))))
        (Transformation|SetActorLocation (Math|Vector|MakeVector (.x _returnvalue_2) (+ _output_get_2 _fixed_y) (.z _returnvalue_2)) true false)
        ;[1 1 1] Setting SlipStream Speed
        (bind _asbp_character_1 (Utilities|Casting|CastToBP_Character1 _player1_2))
        (if (not (Variables|/Game/OurContent/Blueprints/BP_Character1.BP_Character1_C|GetIsZapped _asbp_character_1))
          (if (< (.x (Transformation|GetActorLocation _player1_2)) (.x (Transformation|GetActorLocation _player2_2))) :!label _label
            (Variables|/Script/Engine.CharacterMovementComponent|SetMaxWalkSpeed (Variables|/Script/Engine.Character|GetCharacterMovement _asbp_character_1) (+ (/ (- (.x (Transformation|GetActorLocation (Variables|Default|GetPlayer2))) (.x (Transformation|GetActorLocation (Variables|Default|GetPlayer1)))) 7.0) (Variables|/Script/Engine.CharacterMovementComponent|GetMaxCustomMovementSpeed (Variables|/Script/Engine.Character|GetCharacterMovement _asbp_character_1))))
            (else
              (Variables|/Script/Engine.CharacterMovementComponent|SetMaxWalkSpeed (Variables|/Script/Engine.Character|GetCharacterMovement (stale _asbp_character_2)) (+ (Variables|/Script/Engine.CharacterMovementComponent|GetMaxCustomMovementSpeed (Variables|/Script/Engine.Character|GetCharacterMovement (stale _asbp_character_2))) (/ (- (.x (Transformation|GetActorLocation (Variables|Default|GetPlayer1))) (.x (Transformation|GetActorLocation (Variables|Default|GetPlayer2)))) 7.0))))))
        (else
          (bind _output_get_4 (Variables|Default|SetDistance (- (.x (Transformation|GetActorLocation (Variables|Default|GetPlayer1))) (.x (Transformation|GetActorLocation (Variables|Default|GetPlayer2))))))
          (if (> _output_get_4 3e+02)
            (bind _output_get_5 (Variables|Default|SetYOffSet _output_get_4))
            (Transformation|SetActorLocation (Math|Vector|MakeVector (.x _returnvalue_3) (+ _output_get_5 (Variables|Default|GetFixed%20Y)) (.z _returnvalue_3)) true false)
            (else
              (bind _output_get_6 (Variables|Default|SetYOffSet (Variables|Default|GetFixed%20Y)))
              (Transformation|SetActorLocation (Math|Vector|MakeVector (.x _returnvalue) _output_get_6 (.z _returnvalue)) true false)))
          (bind _asbp_character_2 (Utilities|Casting|CastToBP_Character2 _player2_2))
          (if (not (Variables|/Game/OurContent/Blueprints/BP_Character2.BP_Character2_C|GetIsZapped _asbp_character_2))
            (goto _label)))))))

(event EventBeginPlay
  ;[1 1 1] Comment
  (Utilities|FlowControl|Delay 0.2)
  (Game|Player|SetViewTargetwithBlend (Game|GetPlayerController 0) self 0.0 "VTBlend_Linear" 0.0 false)
  (Variables|Default|SetPlayer1 (Game|GetPlayerCharacter 0))
  (bind _asbp_player_1controller (Utilities|Casting|CastToBP_Player1Controller (Game|GetPlayerController 0)))
  (Variables|Default|SetPlayer2 (Variables|/Game/OurContent/Blueprints/BP_Player1Controller.BP_Player1Controller_C|GetPlayer2CharacterRef _asbp_player_1controller))
  ;[1 1 1] Timer Penalty
  (Utilities|Time|SetTimerbyEvent (delegate Custom|CustomEvent) 1.2e+02))

(fn ConstructionScript)