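; Door Blueprint for the first level, with Open and Close events that slide its left and right door components.
; Open prints a debug string, then plays a timeline once, via DoOnce with no reset, moving only the left door along relative X.
; Close eases both doors to fixed relative positions with MoveComponentTo.
; Older world-space timeline and Lerp logic remains disconnected.
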(event Custom|Open
  (bind _leftdoor (Variables|Default|GetLeftDoor))
  (bind _relativelocation (Variables|/Script/Engine.SceneComponent|GetRelativeLocation _leftdoor))
  (Development|PrintString "Hello")
  (Utilities|FlowControl|DoOnce false
    (:Completed
      (Utilities|FlowControl|Sequence
        (:then_0
          (bind _newtrack_0 (Timeline|NewLeftDoor PlayFromStart)
            (:Update
              (Transformation|SetRelativeLocation _leftdoor (Math|Vector|MakeVector _newtrack_0 (.y _relativelocation) (.z _relativelocation)) false false))))))))

(event Custom|Close
  (Utilities|FlowControl|Sequence
    (:then_0
      (Components|MoveComponentTo (Variables|Default|GetLeftDoor) "0, 0, 0" "0, 0, 0" true true 1.0 false))
    (:then_1
      (Components|MoveComponentTo (Variables|Default|GetRightDoor) "-120.000000,0.000000,0.000000" "0, 0, 0" true true 1.0 false))))

(fn ConstructionScript)