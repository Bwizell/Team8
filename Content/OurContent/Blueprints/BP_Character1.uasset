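; Player 1's character Blueprint for side-to-side movement, jumping and firing one-shot powerups.
; Axis input moves it along world X and records a left/right direction, with the input inverted while IsConfused is set.
; Shoot fires the first held powerup in freeze, zap, confusion order through its component, passing itself and that direction, then clears that powerup's flag.
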(event EventBeginPlay)

(event Collision|EventActorBeginOverlap
  (params (OtherActor :type Actor%20Object%20Reference)))

(event EventTick
  (params (DeltaSeconds :type Float%20%28single-precision%29)))

(event Input|ActionEvents|InputActionJumpPlayer1
  (params (Key :type Key%20Structure :default "None"))
  ;[1 1 1] Inputs for player 1
  (:Pressed
    (Character|Jump)))

(event Input|ActionEvents|InputActionShootPlayer1
  (params (Key :type Key%20Structure :default "None"))
  (bind _leftorright (Variables|Default|GetLeftOrRight))
  ;[1 1 1] Inputs for player 1
  (:Pressed
    (if (Variables|Default|GetHasFreeze)
      (Default|UsePowerupFreeze (Variables|Default|GetBP_FreezeRayComponent) self _leftorright)
      (Variables|Default|SetHasFreeze false)
      (elif (Variables|Default|GetHasZap)
        (Default|UsePowerupZap (Variables|Default|GetBP_ZapGunComponent) self _leftorright)
        (Variables|Default|SetHasZap false)
        (elif (Variables|Default|GetHasConfusion)
          (Default|UsePowerupConf (Variables|Default|GetBP_ConfusionComponent) self (Variables|Default|GetLeftOrRight))
          (Variables|Default|SetHasConfusion false))))))

(event Input|AxisEvents|InputAxisMoveRight/LeftPlayer1
  (params (AxisValue :type Float%20%28single-precision%29))
  (bind _returnvalue (* AxisValue -1.0))
  ;[1 1 1] Inputs for player 1
  (if (Variables|Default|GetIsConfused)
    (Math|Float|CompareFloat _returnvalue 0.0
      (:>
        (Variables|Default|SetLeftOrRight -1.0))
      (:<
        (Variables|Default|SetLeftOrRight 1.0)))
    (Pawn|Input|AddMovementInput "10.000000,0.000000,0.000000" _returnvalue false)
    (else
      (Math|Float|CompareFloat AxisValue 0.0
        (:>
          (Variables|Default|SetLeftOrRight -1.0))
        (:<
          (Variables|Default|SetLeftOrRight 1.0)))
      (Pawn|Input|AddMovementInput "10.000000,0.000000,0.000000" AxisValue false))))

(fn ConstructionScript)