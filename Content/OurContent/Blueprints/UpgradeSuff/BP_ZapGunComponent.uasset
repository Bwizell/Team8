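; Zap gun powerup component that fires a projectile and particle effect to one side of a given actor.
; UsePowerupZap spawns BP_ZapGunParticle and BP_ZapGunProjectile, using the sign of a float to choose negative or positive X and flip rotation; zero spawns nothing.
; Tick keeps the stored particle actor offset beside that actor on the same side, reading the event's parameters directly.
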(event Custom|UsePowerupZap
  (params (NewParam :type Character%20Object%20Reference) (NewParam2 :type Float%20%28double-precision%29))
  (bind _returnvalue (Transformation|GetActorLocation NewParam))
  (bind _returnvalue_2 (+ _returnvalue "0.000000,0.000000,50.000000"))
  (Math|Float|CompareFloat NewParam2 0.0
    (:>
      (bind _returnvalue_3 (Game|SpawnActorfromClass "/Game/OurContent/Blueprints/UpgradeSuff/BP_ZapGunParticle.BP_ZapGunParticle_C" (Math|Transform|MakeTransform _returnvalue_2 "0.000000,180.000000,0.000000" "1.000000,1.000000,1.000000") "Undefined" "MultiplyWithRoot" 0 0))
      (Variables|Default|SetNewVar _returnvalue_3)
      (Game|SpawnActorfromClass "/Game/OurContent/Blueprints/UpgradeSuff/BP_ZapGunProjectile.BP_ZapGunProjectile_C" (Math|Transform|MakeTransform (+ _returnvalue "-100.000000,0.000000,50.000000") "0.000000,180.000000,0.000000" "1.000000,1.000000,1.000000") "Undefined" "MultiplyWithRoot" 0 0))
    (:<
      (bind _returnvalue_4 (Game|SpawnActorfromClass "/Game/OurContent/Blueprints/UpgradeSuff/BP_ZapGunParticle.BP_ZapGunParticle_C" (Math|Transform|MakeTransform _returnvalue_2 "0, 0, 0" "1.000000,1.000000,1.000000") "Undefined" "MultiplyWithRoot" 0 0))
      (Variables|Default|SetNewVar _returnvalue_4)
      (Game|SpawnActorfromClass "/Game/OurContent/Blueprints/UpgradeSuff/BP_ZapGunProjectile.BP_ZapGunProjectile_C" (Math|Transform|MakeTransform (+ _returnvalue "100.000000,0.000000,50.000000") "0, 0, 0" "1.000000,1.000000,1.000000") "Undefined" "MultiplyWithRoot" 0 0))))

(event EventBeginPlay)

(event EventTick
  (params (DeltaSeconds :type Float%20%28single-precision%29))
  (bind _newvar (Variables|Default|GetNewVar))
  (Utilities|IsValid _newvar
    (:Is%20Valid
      (Math|Float|CompareFloat (stale Custom|UsePowerupZap NewParam2) 0.0
        (:>
          (Transformation|SetActorLocation _newvar (+ (Transformation|GetActorLocation (stale Custom|UsePowerupZap NewParam)) "-100.000000,0.000000,50.000000") false false))
        (:<
          (Transformation|SetActorLocation _newvar (+ (Transformation|GetActorLocation (stale Custom|UsePowerupZap NewParam)) "100.000000,0.000000,50.000000") false false))))))