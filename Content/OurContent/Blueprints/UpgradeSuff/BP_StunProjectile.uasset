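; Stun projectile that briefly stuns a BP_Character1 or BP_Character2 entering its sphere.
; It only stuns during its first second, after which an Old flag blocks further hits.
; Each character type has a DoOnce branch that sets IsStunned and disables input for a fraction of a second.
; Input toggling always targets player index 0, via the character for BP_Character1 and the controller for BP_Character2.
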(event OnComponentBeginOverlap(Sphere)
  (params (OverlappedComponent :type Primitive%20Component%20Object%20Reference) (OtherActor :type Actor%20Object%20Reference) (OtherComp :type Primitive%20Component%20Object%20Reference) (OtherBodyIndex :type Integer) (bFromSweep :type Boolean) (SweepResult :type Hit%20Result%20Structure%20%28by%20ref%29))
  (bind _returnvalue (Game|GetPlayerCharacter 0))
  (bind _returnvalue_2 (Game|GetPlayerController 0))
  (if (not (Variables|Default|GetOld))
    (bind _asbp_character_1 (Utilities|Casting|CastToBP_Character1 OtherActor)
      (:then
        (Variables|Default|SetAs%20BP%20Character%201 _asbp_character_1)
        (Utilities|FlowControl|DoOnce false
          (:Completed
            (Input|DisableInput _returnvalue 0)
            (Variables|/Game/OurContent/Blueprints/BP_Character1.BP_Character1_C|SetIs%20stunned (Variables|Default|GetAs%20BP%20Character%201) true)
            (Utilities|FlowControl|Delay 0.3)
            (Input|EnableInput _returnvalue 0)
            (Variables|/Game/OurContent/Blueprints/BP_Character1.BP_Character1_C|SetIs%20stunned (Variables|Default|GetAs%20BP%20Character%201) false))))
      (:CastFailed
        (bind _asbp_character_2 (Utilities|Casting|CastToBP_Character2 OtherActor))
        (Variables|Default|SetAs%20BP%20Character%202 _asbp_character_2)
        (Utilities|FlowControl|DoOnce false
          (:Completed
            (Input|DisableInput _returnvalue_2 0)
            (Variables|/Game/OurContent/Blueprints/BP_Character2.BP_Character2_C|SetIsStunned (Variables|Default|GetAs%20BP%20Character%202) true)
            (Utilities|FlowControl|Delay 0.3)
            (Input|EnableInput _returnvalue_2 0)
            (Variables|/Game/OurContent/Blueprints/BP_Character2.BP_Character2_C|SetIsStunned (Variables|Default|GetAs%20BP%20Character%202) false)))))))

(event EventBeginPlay
  (Utilities|FlowControl|Delay 1.0)
  (Variables|Default|SetOld true))

(event Collision|EventActorBeginOverlap
  (params (OtherActor :type Actor%20Object%20Reference)))

(event EventTick
  (params (DeltaSeconds :type Float%20%28single-precision%29)))

(fn ConstructionScript)