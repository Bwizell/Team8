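; Freeze ray projectile that briefly disables player input on overlap with its sphere.
; Only hits within its first second count, after which an Old flag makes it inert.
; A BP_Character1 hit disables input on that character, while a BP_Character2 hit disables it on player controller 0.
; Each branch re-enables input after a short retriggerable delay.
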(event OnComponentBeginOverlap(Sphere)
  (params (OverlappedComponent :type Primitive%20Component%20Object%20Reference) (OtherActor :type Actor%20Object%20Reference) (OtherComp :type Primitive%20Component%20Object%20Reference) (OtherBodyIndex :type Integer) (bFromSweep :type Boolean) (SweepResult :type Hit%20Result%20Structure%20%28by%20ref%29))
  (bind _returnvalue (Game|GetPlayerController 0))
  (if (not (Variables|Default|GetOld))
    (bind _asbp_character_1 (Utilities|Casting|CastToBP_Character1 OtherActor)
      (:then
        (Input|DisableInput _asbp_character_1 0)
        (Utilities|FlowControl|RetriggerableDelay 0.7)
        (Input|EnableInput OtherActor 0))
      (:CastFailed
        (Utilities|Casting|CastToBP_Character2 OtherActor)
        (Input|DisableInput _returnvalue 0)
        (Utilities|FlowControl|RetriggerableDelay 0.7)
        (Input|EnableInput _returnvalue 0)))))

(event EventBeginPlay
  (Utilities|FlowControl|Delay 1.0)
  (Variables|Default|SetOld true))

(event Collision|EventActorBeginOverlap
  (params (OtherActor :type Actor%20Object%20Reference)))

(event EventTick
  (params (DeltaSeconds :type Float%20%28single-precision%29)))

(fn ConstructionScript)