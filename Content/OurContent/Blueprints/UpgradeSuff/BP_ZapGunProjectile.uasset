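; BP_ZapGunProjectile is the zap gun's projectile, which temporarily slows a player character it touches.
; Its sphere overlap only takes effect during the first half second after spawning, before BeginPlay sets the Old flag.
; A hit on BP_Character1 or BP_Character2 halves walk speed, then restores a hard-coded value after a two-second retriggerable delay running on the projectile.
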(event OnComponentBeginOverlap(Sphere)
  (params (OverlappedComponent :type Primitive%20Component%20Object%20Reference) (OtherActor :type Actor%20Object%20Reference) (OtherComp :type Primitive%20Component%20Object%20Reference) (OtherBodyIndex :type Integer) (bFromSweep :type Boolean) (SweepResult :type Hit%20Result%20Structure%20%28by%20ref%29))
  (if (not (Variables|Default|GetOld))
    (bind _asbp_character_1 (Utilities|Casting|CastToBP_Character1 OtherActor)
      (:then
        (Variables|/Script/Engine.CharacterMovementComponent|SetMaxWalkSpeed (Variables|/Script/Engine.Character|GetCharacterMovement _asbp_character_1) 3e+02)
        (Utilities|FlowControl|RetriggerableDelay 2.0)
        (Variables|/Script/Engine.CharacterMovementComponent|SetMaxWalkSpeed (Variables|/Script/Engine.Character|GetCharacterMovement _asbp_character_1) 6e+02))
      (:CastFailed
        (bind _asbp_character_2 (Utilities|Casting|CastToBP_Character2 OtherActor))
        (Variables|/Script/Engine.CharacterMovementComponent|SetMaxWalkSpeed (Variables|/Script/Engine.Character|GetCharacterMovement _asbp_character_2) 3e+02)
        (Utilities|FlowControl|RetriggerableDelay 2.0)
        (Variables|/Script/Engine.CharacterMovementComponent|SetMaxWalkSpeed (Variables|/Script/Engine.Character|GetCharacterMovement _asbp_character_2) 6e+02)))))

(event EventBeginPlay
  (Utilities|FlowControl|Delay 0.5)
  (Variables|Default|SetOld true))

(event Collision|EventActorBeginOverlap
  (params (OtherActor :type Actor%20Object%20Reference)))

(event EventTick
  (params (DeltaSeconds :type Float%20%28single-precision%29)))

(fn ConstructionScript)