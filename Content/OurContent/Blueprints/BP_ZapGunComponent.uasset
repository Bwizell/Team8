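; Zap gun powerup component that fires a projectile with a freeze-ray particle effect from the actor passed to its use event.
; UsePowerupZap spawns both at that actor's rotation, offsetting the projectile forward or backward on X by checking for a 180-degree facing.
; Tick keeps the stored particle actor at the same facing-dependent offset from that actor, updating location only.
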(event Custom|UsePowerupZap
  (params (NewParam :type Character%20Object%20Reference))
  (bind _returnvalue (Transformation|GetActorRotation NewParam))
  (bind _returnvalue_2 (Transformation|GetActorLocation NewParam))
  (bind _returnvalue_3 (Game|SpawnActorfromClass "/Game/OurContent/Blueprints/BP_FreezeRayParticle.BP_FreezeRayParticle_C" (Math|Transform|MakeTransform (+ _returnvalue_2 "0.000000,0.000000,50.000000") _returnvalue "1.000000,1.000000,1.000000") "Undefined" "MultiplyWithRoot" 0 0))
  (Variables|Default|SetNewVar _returnvalue_3)
  (if (Utilities|Operators|EqualEqual _returnvalue "0.000000,180.000000,0.000000" 0.0001)
    (Game|SpawnActorfromClass "/Game/OurContent/Blueprints/BP_ZapGunProjectile.BP_ZapGunProjectile_C" (Math|Transform|MakeTransform (+ _returnvalue_2 "-100.000000,0.000000,50.000000") _returnvalue "1.000000,1.000000,1.000000") "Undefined" "MultiplyWithRoot" 0 0)
    (else
      (Game|SpawnActorfromClass "/Game/OurContent/Blueprints/BP_ZapGunProjectile.BP_ZapGunProjectile_C" (Math|Transform|MakeTransform (+ _returnvalue_2 "100.000000,0.000000,50.000000") _returnvalue "1.000000,1.000000,1.000000") "Undefined" "MultiplyWithRoot" 0 0))))

(event EventBeginPlay)

(event EventTick
  (params (DeltaSeconds :type Float%20%28single-precision%29))
  (bind _newvar (Variables|Default|GetNewVar))
  (Utilities|IsValid _newvar
    (:Is%20Valid
      (if (Utilities|Operators|EqualEqual (Transformation|GetActorRotation (stale Custom|UsePowerupZap NewParam)) "0.000000,180.000000,0.000000" 0.0001)
        (Transformation|SetActorLocation _newvar (+ (Transformation|GetActorLocation (stale Custom|UsePowerupZap NewParam)) "-100.000000,0.000000,50.000000") false false)
        (else
          (Transformation|SetActorLocation _newvar (+ (Transformation|GetActorLocation (stale Custom|UsePowerupZap NewParam)) "100.000000,0.000000,50.000000") false false))))))