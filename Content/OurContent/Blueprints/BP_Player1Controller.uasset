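; Player controller that creates the main UI, handles pausing, and drives the Player 2 character despite its Player1 name.
; Player 2 axis and action inputs handle horizontal movement and jumping, with movement inverted while confused and facing tracked in LeftOrRight.
; Shoot fires the first held powerup (freeze, zap, then confusion) through its character component and clears it, otherwise falling back to a stun gated by UsedStun.
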(event EventBeginPlay
  ;[1 1 1] Movement for player 2 character
  (bind _returnvalue (UserInterface|CreateWidget "/Game/StarterContent/OurContent/John/MainUI.MainUI_C" self))
  (UserInterface|Viewport|AddtoViewport _returnvalue 0))

(event Input|ActionEvents|InputActionPause
  (params (Key :type Key%20Structure :default "None"))
  (:Pressed
    (Game|SetGamePaused true)
    (Variables|Default|SetbShowMouseCursor true)
    (Utilities|IsValid (Variables|Default|GetPauseMenuRef)
      (:Is%20Valid
        _)
      (:Is%20Not%20Valid
        (bind _returnvalue (UserInterface|CreateWidget "/Game/OurContent/UI/WJ_PauseMenu.WJ_PauseMenu_C"))
        (Variables|Default|SetPauseMenuRef _returnvalue)))
    (UserInterface|Viewport|AddtoViewport (Variables|Default|GetPauseMenuRef) 0)))

(event Input|ActionEvents|InputActionJumpPlayer2
  (params (Key :type Key%20Structure :default "None"))
  ;[1 1 1] Movement for player 2 character
  (:Pressed
    (Character|Jump (Variables|Default|GetPlayer2CharacterRef))))

(event Input|ActionEvents|InputActionShootPlayer2
  (params (Key :type Key%20Structure :default "None"))
  (bind _leftorright (Variables|Default|GetLeftOrRight))
  (bind _player2characterref (Variables|Default|GetPlayer2CharacterRef))
  ;[1 1 1] Movement for player 2 character
  (:Pressed
    (if (Variables|/Game/OurContent/Blueprints/BP_Character2.BP_Character2_C|GetHasFreeze _player2characterref)
      (Default|UsePowerupFreeze (Variables|/Game/OurContent/Blueprints/BP_Character2.BP_Character2_C|GetBP_FreezeRayComponent _player2characterref) _player2characterref _leftorright)
      (Variables|/Game/OurContent/Blueprints/BP_Character2.BP_Character2_C|SetHasFreeze _player2characterref false)
      (Variables|/Game/OurContent/Blueprints/BP_Character2.BP_Character2_C|SetHasPowerup _player2characterref false :!label _label)
      (Variables|/Game/OurContent/Blueprints/BP_Character2.BP_Character2_C|SetActivePowerupImage _player2characterref "")
      (elif (Variables|/Game/OurContent/Blueprints/BP_Character2.BP_Character2_C|GetHasZap _player2characterref)
        (Default|UsePowerupZap (Variables|/Game/OurContent/Blueprints/BP_Character2.BP_Character2_C|GetBP_ZapGunComponent _player2characterref) _player2characterref _leftorright)
        (Variables|/Game/OurContent/Blueprints/BP_Character2.BP_Character2_C|SetHasZap _player2characterref false)
        (goto _label)
        (elif (Variables|/Game/OurContent/Blueprints/BP_Character2.BP_Character2_C|GetHasConfusion _player2characterref)
          (Default|UsePowerupConf (Variables|/Game/OurContent/Blueprints/BP_Character2.BP_Character2_C|GetBP_ConfusionComponent _player2characterref) _player2characterref _leftorright)
          (Variables|/Game/OurContent/Blueprints/BP_Character2.BP_Character2_C|SetHasConfusion _player2characterref false)
          (goto _label)
          (elif (not (Variables|/Game/OurContent/Blueprints/BP_Character2.BP_Character2_C|GetUsedStun _player2characterref))
            (Default|UsePowerupStun (Variables|/Game/OurContent/Blueprints/BP_Character2.BP_Character2_C|GetBP_StunComponent _player2characterref) _player2characterref _leftorright)
            (Variables|/Game/OurContent/Blueprints/BP_Character2.BP_Character2_C|SetUsedStun _player2characterref true)
            (Variables|/Game/OurContent/Blueprints/BP_Character2.BP_Character2_C|SetActivePowerupImage _player2characterref "")
            (Variables|/Game/OurContent/Blueprints/BP_Character2.BP_Character2_C|SetStunTimer _player2characterref 0.0)))))))

(event Input|AxisEvents|InputAxisMoveRight/LeftPlayer2
  (params (AxisValue :type Float%20%28single-precision%29))
  (bind _returnvalue (* AxisValue -1.0))
  (bind _player2characterref (Variables|Default|GetPlayer2CharacterRef))
  ;[1 1 1] Movement for player 2 character
  (if (Variables|/Game/OurContent/Blueprints/BP_Character2.BP_Character2_C|GetIsConfused _player2characterref)
    (Math|Float|CompareFloat _returnvalue 0.0
      (:>
        (Variables|Default|SetLeftOrRight -1.0))
      (:<
        (Variables|Default|SetLeftOrRight 1.0)))
    (Pawn|Input|AddMovementInput _player2characterref "10.000000,0.000000,0.000000" _returnvalue false)
    (else
      (Math|Float|CompareFloat AxisValue 0.0
        (:>
          (Variables|Default|SetLeftOrRight -1.0))
        (:<
          (Variables|Default|SetLeftOrRight 1.0)))
      (Pawn|Input|AddMovementInput _player2characterref "10.000000,0.000000,0.000000" AxisValue false))))

(fn ConstructionScript)