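; Teleporter actor that moves either player character to a destination offset from its own location when it overlaps the Box trigger.
; The overlap casts to BP_Character1, then BP_Character2, and sets that character's location without sweeping.
; If the character's hit-by-other-player flag is set, it also deducts a fixed coin penalty from that character's own counter and clears the flag.
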(event OnComponentBeginOverlap(Box)
  (params (OverlappedComponent :type Primitive%20Component%20Object%20Reference) (OtherActor :type Actor%20Object%20Reference) (OtherComp :type Primitive%20Component%20Object%20Reference) (OtherBodyIndex :type Integer) (bFromSweep :type Boolean) (SweepResult :type Hit%20Result%20Structure%20%28by%20ref%29))
  (bind _returnvalue (Transformation|GetActorLocation))
  (bind _newplayerlocation (Variables|Default|GetNewPlayerLocation))
  (bind _returnvalue_2 (+ _returnvalue _newplayerlocation))
  (bind _asbp_character_1 (Utilities|Casting|CastToBP_Character1 OtherActor)
    (:then
      (Transformation|SetActorLocation _asbp_character_1 _returnvalue_2 false false)
      (if (Variables|/Game/OurContent/Blueprints/BP_Character1.BP_Character1_C|GetHitByOtherPlayer _asbp_character_1)
        (Variables|/Game/OurContent/Blueprints/BP_Character1.BP_Character1_C|SetCoins1 _asbp_character_1 (- (Variables|/Game/OurContent/Blueprints/BP_Character1.BP_Character1_C|GetCoins1 _asbp_character_1) 1e+01))
        (Variables|/Game/OurContent/Blueprints/BP_Character1.BP_Character1_C|SetHitByOtherPlayer _asbp_character_1 false)))
    (:CastFailed
      (bind _asbp_character_2 (Utilities|Casting|CastToBP_Character2 OtherActor))
      (Transformation|SetActorLocation _asbp_character_2 _returnvalue_2 false false)
      (if (Variables|/Game/OurContent/Blueprints/BP_Character2.BP_Character2_C|GetHitbyOtherPlayer _asbp_character_2)
        (Variables|/Game/OurContent/Blueprints/BP_Character2.BP_Character2_C|SetCoins2 _asbp_character_2 (- (Variables|/Game/OurContent/Blueprints/BP_Character2.BP_Character2_C|GetCoins2 _asbp_character_2) 1e+01))
        (Variables|/Game/OurContent/Blueprints/BP_Character2.BP_Character2_C|SetHitbyOtherPlayer _asbp_character_2 false)))))

(event EventBeginPlay)

(event Collision|EventActorBeginOverlap
  (params (OtherActor :type Actor%20Object%20Reference)))

(event EventTick
  (params (DeltaSeconds :type Float%20%28single-precision%29)))

(fn ConstructionScript)