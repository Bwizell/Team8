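; BP_TempCamTest is a test Blueprint that deducts coins from the player once, ten seconds after play begins; despite its name, it contains no camera logic.
; A one-shot timer event casts player character 0 to BP_Character1 and takes 200 from Coins1.
; It then casts the same character to BP_Character2 to reduce Coins2 equally, a step reached only when the first cast succeeds.
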(event Custom|CustomEvent
  (bind _asbp_character_1 (Utilities|Casting|CastToBP_Character1 (Game|GetPlayerCharacter 0)))
  (Variables|/Game/OurContent/Blueprints/BP_Character1.BP_Character1_C|SetCoins1 _asbp_character_1 (- (Variables|/Game/OurContent/Blueprints/BP_Character1.BP_Character1_C|GetCoins1 _asbp_character_1) 2e+02))
  (bind _asbp_character_2 (Utilities|Casting|CastToBP_Character2 (Game|GetPlayerCharacter 0)))
  (Variables|/Game/OurContent/Blueprints/BP_Character2.BP_Character2_C|SetCoins2 _asbp_character_2 (- (Variables|/Game/OurContent/Blueprints/BP_Character2.BP_Character2_C|GetCoins2 _asbp_character_2) 2e+02)))

(event EventBeginPlay
  (Utilities|Time|SetTimerbyEvent (delegate Custom|CustomEvent) 1e+01))

(event Collision|EventActorBeginOverlap
  (params (OtherActor :type Actor%20Object%20Reference)))

(event EventTick
  (params (DeltaSeconds :type Float%20%28single-precision%29)))

(fn ConstructionScript)