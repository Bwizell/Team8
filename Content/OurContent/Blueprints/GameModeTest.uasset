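; Test game mode that sets up two player characters when play begins.
; It spawns BP_Character1 and BP_Character2 at their spawn points, plus a BP_Player2Controller created directly as an actor rather than through a local player.
; It passes the second character and controller references to the existing BP_Player1Controller, then has each controller possess its own character.
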(event EventBeginPlay
  (bind _returnvalue (Game|GetPlayerController 0))
  (bind _spawnpoint2 (Variables|Default|GetSpawnPoint2))
  (bind _returnvalue_2 (Game|SpawnActorfromClass "/Game/OurContent/Blueprints/BP_Character1.BP_Character1_C" (Variables|Default|GetSpawnPoint1) "Undefined" "MultiplyWithRoot" 0 0))
  (bind _returnvalue_3 (Game|SpawnActorfromClass "/Game/OurContent/Blueprints/BP_Character2.BP_Character2_C" _spawnpoint2 "Undefined" "MultiplyWithRoot" 0 0))
  (bind _returnvalue_4 (Game|SpawnActorfromClass "/Game/OurContent/Blueprints/BP_Player2Controller.BP_Player2Controller_C" _spawnpoint2 "Undefined" "MultiplyWithRoot" 0 0))
  (bind _asbp_player_1controller (Utilities|Casting|CastToBP_Player1Controller _returnvalue))
  (Variables|/Game/OurContent/Blueprints/BP_Player1Controller.BP_Player1Controller_C|SetPlayer2CharacterRef _asbp_player_1controller _returnvalue_3)
  (Variables|/Game/OurContent/Blueprints/BP_Player1Controller.BP_Player1Controller_C|SetPlayer2ControllerRef _asbp_player_1controller _returnvalue_4)
  (Pawn|Possess _returnvalue _returnvalue_2)
  (Pawn|Possess _returnvalue_4 _returnvalue_3))

(fn ConstructionScript)